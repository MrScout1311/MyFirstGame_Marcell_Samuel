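; BP_HealthPack is a collectible pickup that heals the third-person player character on touch.
; On actor overlap it casts the other actor to BP_ThirdPersonCharacter and ignores it if health is already at maximum.
; Otherwise it adds a fixed amount of health, pushes the new value to the character's health bar widget, and destroys itself.
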(event `self.ReceiveActorBeginOverlap`
  (params (OtherActor :type "Actor Object Reference"))
  (bind _asbp_third_person_character (cast `/Game/Player/Blueprints/BP_ThirdPersonCharacter` OtherActor))
  (bind _health (`/Game/Player/Blueprints/BP_ThirdPersonCharacter.Health` _asbp_third_person_character))
  (bind _maxhealth (`/Game/Player/Blueprints/BP_ThirdPersonCharacter.MaxHealth` _asbp_third_person_character))
  (if (not (>= _health _maxhealth))
    (`/Game/Player/Blueprints/BP_ThirdPersonCharacter.AddHealth` _asbp_third_person_character 50)
    (`/Game/UserInterface/WBP_HealthBar.SetHealthBarProgress` (`/Game/Player/Blueprints/BP_ThirdPersonCharacter.WBP Health Bar` _asbp_third_person_character) (`KismetMathLibrary.Conv_IntToDouble` _health) (`KismetMathLibrary.Conv_IntToDouble` _maxhealth))
    (`self.K2_DestroyActor`)))

(fn `UserConstructionScript`)