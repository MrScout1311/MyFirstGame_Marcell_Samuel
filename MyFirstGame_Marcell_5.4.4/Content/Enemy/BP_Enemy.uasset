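; Enemy character that patrols random reachable points, chases and shoots the player on sight, and ragdolls when its health runs out.
; PawnSensing interrupts the AIMoveTo patrol loop to start a chase, turning to face the player and calling Shoot.
; Shoot plays a montage and line-traces damage from the muzzle, using a DoOnce reset after the weapon's fire rate.
; Weapon data also supplies mesh and range; health prints every tick.
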(event `self.ReceiveBeginPlay`
  (`self.Patrol`))

(event `self.ReceiveAnyDamage`
  (params (Damage :type "Float (single-precision)") (DamageType :type "DamageType Object Reference") (InstigatedBy :type "Controller Object Reference") (DamageCauser :type "Actor Object Reference"))
  (if (not (`self.IsDeath`))
    (set `self.Health` (- (`self.Health`) Damage))
    (if (<= (`self.Health`) 0)
      (set `self.IsDeath` true)
      (`PrimitiveComponent.SetSimulatePhysics` (`self.Mesh`) true))))

(event `self.ReceiveTick`
  (params (DeltaSeconds :type "Float (single-precision)"))
  (`KismetSystemLibrary.PrintString` (`KismetStringLibrary.Concat_StrStr` "Enemy Health: " (`KismetStringLibrary.Conv_IntToString` (`self.Health`))) true true (struct :`G` 0.66 :`B` 1.0 :`A` 1.0) 0.0001))

(event `Patrol`
  (if (not (`self.IsDeath`))
    (`|AIMoveTo` self (`NavigationSystemV1.K2_GetRandomReachablePointInRadius` (`self.K2_GetActorLocation`) 500.0 null null) null
      (:`OnSuccess`
        _)
      (:`OnFail`
        _))
    (`KismetSystemLibrary.Delay` 2.0)
    (if (not (`self.IsChasingPlayer`))
      (`self.Patrol`))))

(event `self.PawnSensing.OnSeePawn`
  (params (Pawn :type "Pawn Object Reference"))
  (bind _asbp_third_person_character (cast `/Game/Player/Blueprints/BP_ThirdPersonCharacter` Pawn))
  (set `self.IsChasingPlayer` true)
  (`self.Chase Player` _asbp_third_person_character))

(event `Chase Player`
  (params (Player :type "Pawn Object Reference"))
  (if (not (`self.IsDeath`))
    (`|AIMoveTo` self (0.0 0.0 0.0) Player 15.0
      (:`then`
        _)
      (:`OnSuccess`
        (set `self.IsChasingPlayer` false :!label _label))
      (:`OnFail`
        (goto _label)))
    (`self.K2_SetActorRotation` (`KismetMathLibrary.FindLookAtRotation` (`self.K2_GetActorLocation`) (`self.K2_GetActorLocation` Player)))
    (`self.Shoot`)))

(event `Shoot`
  (bind _returnvalue (`SceneComponent.GetSocketLocation` (`self.WeaponMesh`) "MuzzleSocket"))
  (`|ExecutionSequence`
    (:`then_0`
      (`/Engine/EditorBlueprintResources/StandardMacros.DoOnce` false :!label _label_2
        (:`Completed`
          (`|PlayMontage` (`self.Mesh`) "/Game/Enemy/Animation/AM_Shoot.AM_Shoot" 0.5
            (:`then`
              (bind _outhit (`KismetSystemLibrary.LineTraceSingle` :`Start` _returnvalue :`End` (+ _returnvalue (* (`KismetMathLibrary.GetForwardVector` (`self.K2_GetActorRotation`)) (`/Game/Weapon/Blueprint/Data/BP_WeaponData.ShootDistance` (`self.Weapon`)))) :`TraceChannel` "TraceTypeQuery1" :`DrawDebugType` "ForDuration" :`DrawTime` 10.0))
              (bind _asbp_third_person_character (cast `/Game/Player/Blueprints/BP_ThirdPersonCharacter` (`.HitActor` (`GameplayStatics.BreakHitResult` _outhit))))
              (`GameplayStatics.ApplyDamage` _asbp_third_person_character 10.0))))))
    (:`then_1`
      (`KismetSystemLibrary.Delay` (`/Game/Weapon/Blueprint/Data/BP_WeaponData.FireRate` (`self.Weapon`)))
      (goto _label_2 :!via `Reset`))))

(fn `UserConstructionScript`
  (`SkeletalMeshComponent.SetSkeletalMeshAsset` (`self.WeaponMesh`) (`/Game/Weapon/Blueprint/Data/BP_WeaponData.Mesh` (`self.Weapon`))))