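; Enemy spawner actor that spawns BP_Enemy instances at random reachable navmesh points within a fixed radius around itself.
; SpawnEnemy creates a given count at once, lifted above the ground and matching the spawner's rotation.
; BatchSpawnEnemy spawns one enemy per interval through a delay loop until BatchCount runs out or EndSpawn clears IsSpawning.
; The SpawnEnemyPerBatch input is unused.
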(event `SpawnEnemy`
  (params (SpawnEnemyCount :type Integer))
  (set `self.SpawnEnemyCount` SpawnEnemyCount)
  (while (> (`self.SpawnEnemyCount`) 0)
    (`|SpawnActorFromClass` "/Game/Enemy/BP_Enemy.BP_Enemy_C" (`KismetMathLibrary.MakeTransform` (+ (`NavigationSystemV1.K2_GetRandomReachablePointInRadius` (`self.K2_GetActorLocation`) 300.0 null null) (0.0 0.0 100.0)) (`self.K2_GetActorRotation`)) "AdjustIfPossibleButAlwaysSpawn" "MultiplyWithRoot" null null)
    (set `self.SpawnEnemyCount` (- (`self.SpawnEnemyCount`) 1))))

(event `BatchSpawnEnemy`
  (params (BatchCount :type Integer) (SpawnEnemyPerBatch :type Integer) (Interval :type "Float (double-precision)"))
  (set `self.IsSpawning` true)
  (set `self.BatchCount` BatchCount)
  (`|SpawnActorFromClass` "/Game/Enemy/BP_Enemy.BP_Enemy_C" (`KismetMathLibrary.MakeTransform` (`NavigationSystemV1.K2_GetRandomReachablePointInRadius` (`self.K2_GetActorLocation`) 300.0 null null)) "Undefined" "MultiplyWithRoot" null null :!label _label)
  (set `self.BatchCount` (- (`self.BatchCount`) 1))
  (`KismetSystemLibrary.Delay` Interval)
  (if (`self.IsSpawning`)
    (if (> (`self.BatchCount`) 0)
      (goto _label))))

(event `EndSpawn`
  (set `self.IsSpawning` false))

(fn `UserConstructionScript`)