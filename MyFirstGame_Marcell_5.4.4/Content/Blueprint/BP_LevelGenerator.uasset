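; Level generator actor that builds a random tile grid at BeginPlay and places the player on it.
; Each cell of a five-by-five grid spawns a road, building or park tile at random, spaced by a fixed step.
; Road and park positions are collected as candidate spawn transforms, and the player character is then moved to a random one, keeping buildings out of the pool.
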(event `self.ReceiveBeginPlay`
  (for _index (range 5)
    (for _index_2 (range 5)
      (switch `int` (`KismetMathLibrary.RandomIntegerInRange` 0 2)
        (:`0`
          (bind _returnvalue (`KismetMathLibrary.MakeTransform` (`KismetMathLibrary.MakeVector` (`KismetMathLibrary.Conv_IntToDouble` (* _index 400)) (`KismetMathLibrary.Conv_IntToDouble` (* _index_2 400)))))
          (`|SpawnActorFromClass` "/Game/Blueprint/BP_Tile_Road.BP_Tile_Road_C" _returnvalue "Undefined" "MultiplyWithRoot" null null)
          (`KismetArrayLibrary.Array_Add` (`|MakeArray` (`self.SpawnPlayer`)) _returnvalue))
        (:`1`
          (`|SpawnActorFromClass` "/Game/Blueprint/BP_Tile_Building.BP_Tile_Building_C" _returnvalue "Undefined" "MultiplyWithRoot" null null))
        (:`2`
          (`|SpawnActorFromClass` "/Game/Blueprint/BP_Tile_Park.BP_Tile_Park_C" _returnvalue "Undefined" "MultiplyWithRoot" null null)
          (`KismetArrayLibrary.Array_Add` (`|MakeArray` (`self.SpawnPlayer`)) _returnvalue)))))
  (`self.K2_SetActorTransform` (`GameplayStatics.GetPlayerCharacter` 0) (`KismetArrayLibrary.Array_Random` (`|MakeArray` (`self.SpawnPlayer`))) false false))

(fn `UserConstructionScript`)